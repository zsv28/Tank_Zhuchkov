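; BP_PawnTank is the tank pawn Blueprint, which wires player input to UI and interaction.
; BeginPlay adds the minimap widget, and hardcoded keys open the inventory, a spawned-list widget, and a save/load menu that pauses the game and shows the cursor.
; Input actions trigger Interaction and toggle quest list visibility, calling functions defined outside these graphs.
; An unconnected chain for showing WBP_TankInfo through MyHUD never runs.
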(event EventBeginPlay
  (Utilities|FlowControl|Sequence
    (:then_1
      (bind _returnvalue (UserInterface|CreateWidget "/Game/UI/Widgets/MiniMap/WBP_MiniMap.WBP_MiniMap_C" (Game|GetPlayerController 0)))
      (UserInterface|Viewport|AddtoViewport _returnvalue 0))))

(event Collision|EventActorBeginOverlap
  (params (OtherActor :type Actor%20Object%20Reference)))

(event EventTick
  (params (DeltaSeconds :type Float%20%28single-precision%29)))

(event Input|ActionEvents|InputActionInteract
  (params (Key :type Key%20Structure :default "None"))
  ;[0 1 0.02932] Interact
  (:Pressed
    (Class|InteractionComponent|Interact (Variables|Default|GetInteraction))))

(event Input|ActionEvents|InputActionToggleQuestList
  (params (Key :type Key%20Structure :default "None"))
  (:Pressed
    (Class|TankPawn|ToggleQuestListVisibility)))

(event Input|KeyboardEvents|K
  (params (Key :type Key%20Structure :default "None"))
  (:Pressed
    (bind _returnvalue (UserInterface|CreateWidget "/Game/UI/Widgets/WBP_SpawnedList.WBP_SpawnedList_C" (Game|GetPlayerController 0)))
    (UserInterface|Viewport|AddtoViewport _returnvalue 0)))

(event Input|KeyboardEvents|C
  (params (Key :type Key%20Structure :default "None"))
  (:Pressed
    (Class|TankPawn|EnableInventary)))

(event Input|KeyboardEvents|Q
  (params (Key :type Key%20Structure :default "None"))
  (bind _returnvalue (Game|GetPlayerController 0))
  (:Pressed
    (bind _returnvalue_2 (UserInterface|CreateWidget "/Game/UI/Widgets/WBP_Save_Load.WBP_Save_Load_C" _returnvalue))
    (UserInterface|Viewport|AddtoViewport _returnvalue_2 0)
    (Game|SetGamePaused true)
    (Variables|/Script/Engine.PlayerController|SetbShowMouseCursor _returnvalue true)))

(fn ConstructionScript)