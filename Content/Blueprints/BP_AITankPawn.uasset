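; BP_AITankPawn is the Blueprint pawn for an AI-controlled tank.
; On BeginPlay it runs the parent logic, then casts the Health component's widget to WBP_HUD_Enemy_Health and passes itself in as that widget's BPBasePawn reference.
; The construction script only calls the parent, and the Tick and overlap events are disabled stubs.
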(event EventBeginPlay
  (|CallParentFunction)
  ;[0.6266 1 0.6275] HUD_AI_Health
  (bind _aswbp_hud_enemy_health (Utilities|Casting|CastToWBP_HUD_Enemy_Health (UserInterface|GetUserWidgetObject (Variables|Default|Gethealth))))
  (Variables|/Game/UI/Widgets/WBP_HUD_Enemy_Health.WBP_HUD_Enemy_Health_C|SetBP_BasePawn _aswbp_hud_enemy_health self))

(event Collision|EventActorBeginOverlap
  (params (OtherActor :type Actor%20Object%20Reference))
  (|CallParentFunction OtherActor) ; This node is disabled and will not be called.\nDrag off pins to build functionality.
)

(event EventTick
  (params (DeltaSeconds :type Float%20%28single-precision%29))
  (|CallParentFunction DeltaSeconds) ; This node is disabled and will not be called.\nDrag off pins to build functionality.
)

(fn ConstructionScript
  (|CallParentFunction))